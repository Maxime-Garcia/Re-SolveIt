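; BP_GreenButton is a one-shot trigger that turns a BP_Ball green when the ball overlaps its Sphere.
; The overlap sets the ball mesh to the green material, enables custom depth with a stencil value, tags the ball "Green" and plays a button sound.
; The button then shows an off material on its Cylinder and disables Sphere collision so it cannot fire again.
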(event `self.Sphere.OnComponentBeginOverlap`
  (params (OverlappedComponent :type "PrimitiveComponent Object Reference") (OtherActor :type "Actor Object Reference") (OtherComp :type "PrimitiveComponent Object Reference") (OtherBodyIndex :type Integer) (bFromSweep :type Boolean) (SweepResult :type "HitResult Structure (by ref)"))
  (bind _asbp_ball (cast `/Game/BP_Ball` OtherActor))
  (bind _ballmesh (`/Game/BP_Ball.BallMesh` _asbp_ball))
  (`PrimitiveComponent.SetMaterial` _ballmesh 0 "/Game/Materials/M_Green.M_Green")
  (`PrimitiveComponent.SetRenderCustomDepth` _ballmesh true)
  (`PrimitiveComponent.SetCustomDepthStencilValue` _ballmesh 1)
  (`GameplayStatics.PlaySound2D` "/Game/Buttons/ButtonSound.ButtonSound" 1.0 1.0 0.0 null null)
  (`KismetArrayLibrary.Array_Add` (`Actor.Tags` _asbp_ball) "Green")
  (`PrimitiveComponent.SetMaterial` (`self.Cylinder`) 0 "/Game/Materials/M_OffColor.M_OffColor")
  (`PrimitiveComponent.SetCollisionEnabled` (`self.Sphere`) "NoCollision"))

(fn `UserConstructionScript`)