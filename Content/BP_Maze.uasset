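; Maze board actor that the player tilts on two axes, with input for pausing and restarting the level.
; TiltForward adds world pitch and TiltRight adds local roll to BoardMesh, scaled by RotationSpeed.
; After each step the changed angle is clamped between MinClamp and MaxClamp, pitch in world space and roll in relative space.
; Pause toggles game pause through IsPaused, and Reload reopens the Maze1 level.
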(event `InputAxis|TiltForward`
  (params (AxisValue :type "Float (single-precision)"))
  (bind (_returnvalue_roll _returnvalue_pitch _returnvalue_yaw) (`KismetMathLibrary.BreakRotator` (`SceneComponent.K2_GetComponentRotation` (`self.BoardMesh`))))
  (`SceneComponent.K2_AddWorldRotation` (`self.BoardMesh`) (`KismetMathLibrary.MakeRotator` 0.0 (* AxisValue (`self.RotationSpeed`))) false false)
  (`SceneComponent.K2_SetWorldRotation` (`self.BoardMesh`) (`KismetMathLibrary.MakeRotator` _returnvalue_roll (`KismetMathLibrary.FClamp` _returnvalue_pitch (`self.MinClamp`) (`self.MaxClamp`)) _returnvalue_yaw) false false))

(event `InputAxis|TiltRight`
  (params (AxisValue :type "Float (single-precision)"))
  (bind _boardmesh (`self.BoardMesh`))
  (bind (_relativerotation_roll _relativerotation_pitch _relativerotation_yaw) (`KismetMathLibrary.BreakRotator` (`SceneComponent.RelativeRotation` _boardmesh)))
  (`SceneComponent.K2_AddLocalRotation` (`self.BoardMesh`) (`KismetMathLibrary.MakeRotator` (* AxisValue (`self.RotationSpeed`))) false false)
  (`SceneComponent.K2_SetRelativeRotation` _boardmesh (`KismetMathLibrary.MakeRotator` (`KismetMathLibrary.FClamp` _relativerotation_roll (`self.MinClamp`) (`self.MaxClamp`)) _relativerotation_pitch _relativerotation_yaw) false false))

(event `InputAction|Pause` :paused true
  (params (Key :type "Key Structure"))
  (:`Pressed`
    (if (`self.IsPaused`)
      (set `self.IsPaused` false)
      (`GameplayStatics.SetGamePaused` false)
      (else
        (set `self.IsPaused` true)
        (`GameplayStatics.SetGamePaused` true)))))

(event `InputAction|Reload`
  (params (Key :type "Key Structure"))
  (:`Pressed`
    (`GameplayStatics.OpenLevelBySoftObjectPtr` "/Game/StarterContent/Maps/Maze1.Maze1")))

(fn `UserConstructionScript`)