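; Rolling physics ball for a tilt-maze game that mixes colors and reloads Maze1 when it leaves its height limits.
; A fast looping timer merges primary color tags into secondaries or white, setting material and custom depth stencil, though Magenta uses the cyan material.
; Mesh hits scale the rolling sound volume by horizontal speed.
; ResetBall and ResetMap exist, but their event graph calls are unwired.
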(event `CheckColors`
  (bind _ballmesh (`self.BallMesh`))
  (bind _ballmesh_2 (`self.BallMesh`))
  (bind _ballmesh_3 (`self.BallMesh`))
  (bind _ballmesh_4 (`self.BallMesh`))
  (bind _tags (`self.Tags`))
  (bind _tags_2 (`self.Tags`))
  (bind _tags_3 (`self.Tags`))
  (bind _tags_4 (`self.Tags`))
  (bind _tags_5 (`self.Tags`))
  (bind _tags_6 (`self.Tags`))
  (`|ExecutionSequence`
    (:`then_0`
      ;[1 1 1] Red & Green & Blue => White
      (if (and (`self.ActorHasTag` "Red") (`self.ActorHasTag` "Cyan"))
        (`KismetArrayLibrary.Array_RemoveItem` _tags_5 "Red")
        (`KismetArrayLibrary.Array_RemoveItem` _tags_5 "Cyan")
        (`KismetArrayLibrary.Array_Add` _tags_5 "White")
        ;[1 1 1] Red & Green & Blue => White
        (`PrimitiveComponent.SetMaterial` _ballmesh_3 0 "/Game/Materials/M_White.M_White" :!label _label)
        (`PrimitiveComponent.SetRenderCustomDepth` _ballmesh_3 true)
        (`PrimitiveComponent.SetCustomDepthStencilValue` _ballmesh_3 6)))
    (:`then_1`
      (if (and (`self.ActorHasTag` "Blue") (`self.ActorHasTag` "Yellow"))
        (`KismetArrayLibrary.Array_RemoveItem` _tags_6 "Blue")
        (`KismetArrayLibrary.Array_RemoveItem` _tags_6 "Yellow")
        (`KismetArrayLibrary.Array_Add` _tags_6 "White")
        (goto _label)))
    (:`then_2`
      ;[1 1 1] Red & Green & Blue => White
      (if (and (`self.ActorHasTag` "Magenta") (`self.ActorHasTag` "Green"))
        (`KismetArrayLibrary.Array_RemoveItem` _tags "Magenta")
        (`KismetArrayLibrary.Array_RemoveItem` _tags "Green")
        (`KismetArrayLibrary.Array_Add` _tags "White")
        (goto _label)))
    (:`then_3`
      ;[0 0.7443 1] Blue & Green => Cyan
      (if (and (`self.ActorHasTag` "Blue") (`self.ActorHasTag` "Green"))
        (`KismetArrayLibrary.Array_RemoveItem` _tags_3 "Green")
        (`KismetArrayLibrary.Array_RemoveItem` _tags_3 "Blue")
        (`KismetArrayLibrary.Array_Add` _tags_3 "Cyan")
        (`PrimitiveComponent.SetMaterial` _ballmesh_2 0 "/Game/Materials/M_Cyan.M_Cyan")
        (`PrimitiveComponent.SetRenderCustomDepth` _ballmesh_2 true)
        (`PrimitiveComponent.SetCustomDepthStencilValue` _ballmesh_2 3)))
    (:`then_4`
      ;[0.9717 0 1] Blue & Red => Magenta
      (if (and (`self.ActorHasTag` "Blue") (`self.ActorHasTag` "Red"))
        (`KismetArrayLibrary.Array_RemoveItem` _tags_4 "Red")
        (`KismetArrayLibrary.Array_RemoveItem` _tags_4 "Blue")
        (`KismetArrayLibrary.Array_Add` _tags_4 "Magenta")
        (`PrimitiveComponent.SetMaterial` _ballmesh 0 "/Game/Materials/M_Cyan.M_Cyan")
        (`PrimitiveComponent.SetRenderCustomDepth` _ballmesh true)
        (`PrimitiveComponent.SetCustomDepthStencilValue` _ballmesh 5)))
    (:`then_5`
      ;[1 0.971 0] Green & Red => Yellow
      (if (and (`self.ActorHasTag` "Green") (`self.ActorHasTag` "Red"))
        (`KismetArrayLibrary.Array_RemoveItem` _tags_2 "Red")
        (`KismetArrayLibrary.Array_RemoveItem` _tags_2 "Green")
        (`KismetArrayLibrary.Array_Add` _tags_2 "Yellow")
        (`PrimitiveComponent.SetMaterial` _ballmesh_4 0 "/Game/Materials/M_Yellow.M_Yellow")
        (`PrimitiveComponent.SetRenderCustomDepth` _ballmesh_4 true)
        (`PrimitiveComponent.SetCustomDepthStencilValue` _ballmesh_4 4)))))

(event `self.ReceiveBeginPlay`
  (`AudioComponent.Play` (`self.BallRollSound`) 0.0)
  (set `self.StartingLocation` (`self.K2_GetActorLocation`))
  (`KismetSystemLibrary.K2_SetTimerDelegate` (delegate `CheckColors`) 0.01 true))

(event `self.ReceiveTick`
  (params (DeltaSeconds :type "Float (single-precision)"))
  (bind (_returnvalue_x _returnvalue_y _returnvalue_z) (`KismetMathLibrary.BreakVector` (`self.K2_GetActorLocation`)))
  (if (or (> _returnvalue_z (`self.KillHeightUp`)) (< _returnvalue_z (`self.KillHeightDown`)))
    (`GameplayStatics.OpenLevelBySoftObjectPtr` "/Game/StarterContent/Maps/Maze1.Maze1")))

(event `self.BallMesh.OnComponentHit`
  (params (HitComponent :type "PrimitiveComponent Object Reference") (OtherActor :type "Actor Object Reference") (OtherComp :type "PrimitiveComponent Object Reference") (NormalImpulse :type "Vector Structure") (Hit :type "HitResult Structure (by ref)"))
  ;[1 1 1] Rolling Sound
  (bind _returnvalue (`PrimitiveComponent.GetPhysicsLinearVelocity` (`self.BallMesh`) "None"))
  (`|ExecutionSequence`
    (:`then_0`
      (`/Engine/EditorBlueprintResources/StandardMacros.CompareFloat` (.z _returnvalue) 2.0))
    (:`then_1`
      (`AudioComponent.SetVolumeMultiplier` (`self.BallRollSound`) (/ (`KismetMathLibrary.VSizeXY` _returnvalue) 300.0)))))

(fn `ResetBall`
  (`self.K2_SetActorLocation` (`self.StartingLocation`))
  (`PrimitiveComponent.SetPhysicsLinearVelocity` (`self.BallMesh`) (0.0 0.0 0.0) false "None"))

(fn `ResetMap`
  (bind _returnvalue (`GameplayStatics.GetActorOfClass` "/Game/BP_Maze.BP_Maze_C"))
  (`SceneComponent.K2_SetWorldRotation` :`self` (`/Game/BP_Maze.BoardMesh` _returnvalue)))

(fn `UserConstructionScript`)