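; BP_BlueDoor is a door that opens only for a ball tagged Blue.
; When its static mesh is hit by such a BP_Ball, it plays a 2D sound, disables the mesh's collision and swaps to an activated material.
; It then finds the first top-level WBP_Timer widget and increments its Timer value directly, with no check that one exists.
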(event `self.StaticMesh.OnComponentHit`
  (params (HitComponent :type "PrimitiveComponent Object Reference") (OtherActor :type "Actor Object Reference") (OtherComp :type "PrimitiveComponent Object Reference") (NormalImpulse :type "Vector Structure") (Hit :type "HitResult Structure (by ref)"))
  (bind _asbp_ball (cast `/Game/BP_Ball` OtherActor))
  (if (`self.ActorHasTag` _asbp_ball "Blue")
    (`GameplayStatics.PlaySound2D` "/Game/ActivatedSound.ActivatedSound" 1.0 1.0 0.0 null null)
    (`PrimitiveComponent.SetCollisionEnabled` (`self.StaticMesh`) "NoCollision")
    (`PrimitiveComponent.SetMaterial` (`self.StaticMesh`) 0 "/Game/Materials/M_BlueActivated.M_BlueActivated")
    (bind _foundwidgets (`WidgetBlueprintLibrary.GetAllWidgetsOfClass` "/Game/WBP_Timer.WBP_Timer_C"))
    (bind _output (`|GetArrayItem` _foundwidgets))
    (set `/Game/WBP_Timer.Timer` (+ (`/Game/WBP_Timer.Timer` _output) 1) _output)))

(fn `UserConstructionScript`)